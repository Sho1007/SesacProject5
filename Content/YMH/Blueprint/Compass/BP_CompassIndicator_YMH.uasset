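; BP_CompassIndicator_YMH is a component that adds an icon for its owning actor to the player's compass HUD.
; On BeginPlay or InitWidget, Wayout owners qualify by a name substring match in the player's EscapeComponent exit array.
; Other owners qualify when their ObjectiveIndicator ObjectID matches an objective in the quest log.
; Each match creates a compass icon widget under the CompassOverlay; the server RPC is an empty stub.
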(event Custom|InitWidget
  (bind _returnvalue (Components|GetOwner))
  (bind _returnvalue_2 (Actor|GetComponentbyClass _returnvalue "/Game/YMH/Blueprint/QuestSystem/BP_ObjectiveIndicator_YMH.BP_ObjectiveIndicator_YMH_C"))
  (bind _ascharacter_base (Utilities|Casting|CastToCharacterBase (Game|GetPlayerCharacter 0)))
  (Utilities|IsValid _ascharacter_base
    (:Is%20Valid
      (if (Variables|Default|GetbWayout)
        (for _array_element (Class|EscapeComponent|GetExitArray (Actor|GetComponentbyClass _ascharacter_base "/Script/SesacProject5.EscapeComponent"))
          (if (Utilities|String|Contains (Utilities|String|ToString(Object) _array_element) (Utilities|String|ToString(Object) (Components|GetOwner self)))
            (bind _returnvalue_3 (UserInterface|CreateWidget "/Game/YMH/Blueprint/Compass/WBP_CompassIcon_YMH.WBP_CompassIcon_YMH_C" 0 (Variables|Default|GetIcon) (Components|GetOwner)))
            (Widget|Panel|AddChild (Variables|/Game/YMH/Blueprint/Compass/WBP_Compass_YMH.WBP_Compass_YMH_C|GetCompassOverlay (Variables|/Game/YMH/Blueprint/Compass/WBP_CompassHUD_YMH.WBP_CompassHUD_YMH_C|GetWBP_Compass_YMH (Variables|/Game/YMH/Blueprint/Compass/BP_CompassComp_YMH.BP_CompassComp_YMH_C|GetCompassHUD (Actor|GetComponentbyClass _ascharacter_base "/Game/YMH/Blueprint/Compass/BP_CompassComp_YMH.BP_CompassComp_YMH_C")))) _returnvalue_3)))
        (else
          (Utilities|IsValid _returnvalue_2
            (:Is%20Valid
              (for _array_element_2 (Variables|/Script/SesacProject5.QuestLogComponent|GetquestList (Actor|GetComponentbyClass _ascharacter_base "/Game/YMH/Blueprint/QuestSystem/BP_QuestLogComponent_YMH.BP_QuestLogComponent_YMH_C"))
                (for _array_element_3 (Utilities|Struct|BreakQuestDetails (Utilities|Struct|BreakQuestManagement _array_element_2))
                  (for _array_element_4 (Utilities|Struct|BreakStageDetails _array_element_3)
                    (if (Utilities|Enum|Equal(Enum) (Variables|/Script/SesacProject5.ObjectiveComponent|GetobjectID _returnvalue_2) (Utilities|Struct|BreakObjectiveDetails _array_element_4))
                      (bind _returnvalue_4 (UserInterface|CreateWidget "/Game/YMH/Blueprint/Compass/WBP_CompassIcon_YMH.WBP_CompassIcon_YMH_C" 0 (Variables|Default|GetIcon) (Components|GetOwner)))
                      (Widget|Panel|AddChild (Variables|/Game/YMH/Blueprint/Compass/WBP_Compass_YMH.WBP_Compass_YMH_C|GetCompassOverlay (Variables|/Game/YMH/Blueprint/Compass/WBP_CompassHUD_YMH.WBP_CompassHUD_YMH_C|GetWBP_Compass_YMH (Variables|/Game/YMH/Blueprint/Compass/BP_CompassComp_YMH.BP_CompassComp_YMH_C|GetCompassHUD (Actor|GetComponentbyClass _ascharacter_base "/Game/YMH/Blueprint/Compass/BP_CompassComp_YMH.BP_CompassComp_YMH_C")))) _returnvalue_4))))))))))))

(event Custom|ServerRPC_InitWidget)

(event EventBeginPlay
  (bind _returnvalue (Components|GetOwner))
  (bind _returnvalue_2 (Actor|GetComponentbyClass _returnvalue "/Game/YMH/Blueprint/QuestSystem/BP_ObjectiveIndicator_YMH.BP_ObjectiveIndicator_YMH_C"))
  (bind _ascharacter_base (Utilities|Casting|CastToCharacterBase (Game|GetPlayerCharacter 0)))
  (Utilities|IsValid _ascharacter_base
    (:Is%20Valid
      (if (Variables|Default|GetbWayout)
        (for _array_element (Class|EscapeComponent|GetExitArray (Actor|GetComponentbyClass _ascharacter_base "/Script/SesacProject5.EscapeComponent"))
          (if (Utilities|String|Contains (Utilities|String|ToString(Object) _array_element) (Utilities|String|ToString(Object) (Components|GetOwner self)))
            (bind _returnvalue_3 (UserInterface|CreateWidget "/Game/YMH/Blueprint/Compass/WBP_CompassIcon_YMH.WBP_CompassIcon_YMH_C" 0 (Variables|Default|GetIcon) (Components|GetOwner)))
            (Widget|Panel|AddChild (Variables|/Game/YMH/Blueprint/Compass/WBP_Compass_YMH.WBP_Compass_YMH_C|GetCompassOverlay (Variables|/Game/YMH/Blueprint/Compass/WBP_CompassHUD_YMH.WBP_CompassHUD_YMH_C|GetWBP_Compass_YMH (Variables|/Game/YMH/Blueprint/Compass/BP_CompassComp_YMH.BP_CompassComp_YMH_C|GetCompassHUD (Actor|GetComponentbyClass _ascharacter_base "/Game/YMH/Blueprint/Compass/BP_CompassComp_YMH.BP_CompassComp_YMH_C")))) _returnvalue_3)))
        (else
          (Utilities|IsValid _returnvalue_2
            (:Is%20Valid
              (for _array_element_2 (Variables|/Script/SesacProject5.QuestLogComponent|GetquestList (Actor|GetComponentbyClass _ascharacter_base "/Game/YMH/Blueprint/QuestSystem/BP_QuestLogComponent_YMH.BP_QuestLogComponent_YMH_C"))
                (for _array_element_3 (Utilities|Struct|BreakQuestDetails (Utilities|Struct|BreakQuestManagement _array_element_2))
                  (for _array_element_4 (Utilities|Struct|BreakStageDetails _array_element_3)
                    (if (Utilities|Enum|Equal(Enum) (Variables|/Script/SesacProject5.ObjectiveComponent|GetobjectID _returnvalue_2) (Utilities|Struct|BreakObjectiveDetails _array_element_4))
                      (bind _returnvalue_4 (UserInterface|CreateWidget "/Game/YMH/Blueprint/Compass/WBP_CompassIcon_YMH.WBP_CompassIcon_YMH_C" 0 (Variables|Default|GetIcon) (Components|GetOwner)))
                      (Widget|Panel|AddChild (Variables|/Game/YMH/Blueprint/Compass/WBP_Compass_YMH.WBP_Compass_YMH_C|GetCompassOverlay (Variables|/Game/YMH/Blueprint/Compass/WBP_CompassHUD_YMH.WBP_CompassHUD_YMH_C|GetWBP_Compass_YMH (Variables|/Game/YMH/Blueprint/Compass/BP_CompassComp_YMH.BP_CompassComp_YMH_C|GetCompassHUD (Actor|GetComponentbyClass _ascharacter_base "/Game/YMH/Blueprint/Compass/BP_CompassComp_YMH.BP_CompassComp_YMH_C")))) _returnvalue_4))))))))))))